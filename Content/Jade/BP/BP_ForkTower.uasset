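; BP_ForkTower is an interactable music tower that the player activates in a four-step sequence.
; Box overlap shows an E prompt and gates EFork, which fires once to play the tower's sound and visualizer and increment FirstPerson's ForkCount.
; The first three activations reveal a Line and raise the next tagged tower by timeline.
; The fourth messages BP_Pawn_Music, hides path tracers and, after a delay, fades all tower audio.
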(event OnComponentBeginOverlap(Box)
  (params (OverlappedComponent :type Primitive%20Component%20Object%20Reference) (OtherActor :type Actor%20Object%20Reference) (OtherComp :type Primitive%20Component%20Object%20Reference) (OtherBodyIndex :type Integer) (bFromSweep :type Boolean) (SweepResult :type Hit%20Result%20Structure%20%28by%20ref%29))
  (Utilities|Casting|CastToFirstPerson OtherActor)
  (if (Variables|Default|GetCan_Active)
    (Utilities|FlowControl|DoOnce false
      (:Completed
        (bind _returnvalue (UserInterface|CreateWidget "/Game/Jade/Widget/PressE_Interct.PressE_Interct_C"))
        (UserInterface|Viewport|AddtoViewport _returnvalue 0)
        (Utilities|FlowControl|Gate true) ; enters at Open
      ))))

(event OnComponentEndOverlap(Box)
  (params (OverlappedComponent :type Primitive%20Component%20Object%20Reference) (OtherActor :type Actor%20Object%20Reference) (OtherComp :type Primitive%20Component%20Object%20Reference) (OtherBodyIndex :type Integer))
  (Utilities|Casting|CastToFirstPerson OtherActor)
  (if (Variables|Default|GetCan_Active)
    (Utilities|FlowControl|Sequence
      (:then_0
        (Utilities|FlowControl|DoOnce false) ; enters at Reset
      )
      (:then_1
        (Widget|RemovefromParent (stale OnComponentBeginOverlap(Box) _returnvalue))
        (Utilities|FlowControl|Gate true) ; enters at Close
      ))))

(event EventBeginPlay)

(event EventEFork
  (Utilities|FlowControl|Gate true
    (:Exit
      (Utilities|FlowControl|DoOnce false
        (:Completed
          (Viewport|RemoveAllWidgets)
          ;[1 1 1] 音乐
          (Audio|Components|Audio|Play (Variables|Default|GetCybird-4jianzhu-lead) 0.0)
          (Rendering|SetVisibility (Variables|Default|GetP_ElectricOrb) true false)
          ;[1 1 1] 判断点塔数量
          (bind _outactors (Actor|GetAllActorsOfClass "/Game/PUPI/Demo/Character/FirstPerson.FirstPerson_C"))
          (bind _output_get (Variables|/Game/PUPI/Demo/Character/FirstPerson.FirstPerson_C|SetFork_Count (Utilities|Array|Get(acopy) _outactors) (+ (stale _output_get) 1)))
          (if (== _output_get 1)
            ;[1 1 1] TA1 Rise
            (bind _outactors_2 (Actor|GetAllActorsOfClasswithTag "BP_ForkTower_C" "TA1"))
            (Rendering|SetActorHiddenInGame (Variables|Default|GetLine) false)
            (Audio|PlaySound2D "/Game/sound/In_the_distant_echo.In_the_distant_echo" 1.0 1.0 0.0 0 0)
            (Variables|Default|SetReturn%20Value%20Z1 (.z (Transformation|GetActorLocation (Utilities|Array|Get(acopy) _outactors_2))))
            (bind _新建轨道_0 (Timeline|时间轴 Play)
              (:Update
                (Transformation|SetActorLocation (Utilities|Array|Get(acopy) _outactors_2) (Math|Vector|MakeVector (.x (Transformation|GetActorLocation (Utilities|Array|Get(acopy) _outactors_2))) (.y (Transformation|GetActorLocation (Utilities|Array|Get(acopy) _outactors_2))) (Math|Float|Lerp (Variables|Default|GetReturn%20Value%20Z1) (+ (Variables|Default|GetReturn%20Value%20Z1) 5e+02) _新建轨道_0)) false false)))
            (elif (== _output_get 2)
              ;[1 1 1] TA2 Rise
              (bind _outactors_3 (Actor|GetAllActorsOfClasswithTag "BP_ForkTower_C" "TA2"))
              (Rendering|SetActorHiddenInGame (Variables|Default|GetLine) false)
              (Variables|Default|SetReturn%20Value%20Z2 (.z (Transformation|GetActorLocation (Utilities|Array|Get(acopy) _outactors_3))))
              (bind _新建轨道_0_2 (Timeline|时间轴_0 Play)
                (:Update
                  (Transformation|SetActorLocation (Utilities|Array|Get(acopy) _outactors_3) (Math|Vector|MakeVector (.x (Transformation|GetActorLocation (Utilities|Array|Get(acopy) _outactors_3))) (.y (Transformation|GetActorLocation (Utilities|Array|Get(acopy) _outactors_3))) (Math|Float|Lerp (Variables|Default|GetReturn%20Value%20Z2) (+ (Variables|Default|GetReturn%20Value%20Z2) 5e+02) _新建轨道_0_2)) false false)))
              (elif (== _output_get 3)
                ;[1 1 1] TA3 Rise
                (bind _outactors_4 (Actor|GetAllActorsOfClasswithTag "BP_ForkTower_C" "TA3"))
                (Rendering|SetActorHiddenInGame (Variables|Default|GetLine) false)
                (Variables|Default|SetReturn%20Value%20Z3 (.z (Transformation|GetActorLocation (Utilities|Array|Get(acopy) _outactors_4))))
                (bind _新建轨道_0_3 (Timeline|时间轴_1 Play)
                  (:Update
                    (Transformation|SetActorLocation (Utilities|Array|Get(acopy) _outactors_4) (Math|Vector|MakeVector (.x (Transformation|GetActorLocation (Utilities|Array|Get(acopy) _outactors_4))) (.y (Transformation|GetActorLocation (Utilities|Array|Get(acopy) _outactors_4))) (Math|Float|Lerp (Variables|Default|GetReturn%20Value%20Z3) (+ (Variables|Default|GetReturn%20Value%20Z3) 5e+02) _新建轨道_0_3)) false false)))
                (elif (== _output_get 4)
                  (bind _outactors_5 (Actor|GetAllActorsOfClass "/Game/Jade/BP/BP_Pawn_Music.BP_Pawn_Music_C"))
                  (Class|BIFirstperson|ForkCom(Message) _outactors_5)
                  (bind _outactors_6 (Actor|GetAllActorsOfClass "/Game/PathTracer/Blueprints/BP_PathTracer.BP_PathTracer_C"))
                  (Rendering|SetActorHiddenInGame _outactors_6 true)
                  ;[1 1 1] 延迟两秒，停止播放
                  (Utilities|FlowControl|Delay 2.0)
                  (bind _outactors_7 (Actor|GetAllActorsOfClass "BP_ForkTower_C"))
                  (for _array_element _outactors_7
                    (Audio|Components|Audio|FadeOut (Variables|BP_ForkTower_C|GetCybird-4jianzhu-lead _array_element) 2.0 0.0 "Linear" :!class /Script/Engine.AudioComponent)))))))))))

(fn ConstructionScript
  (Variables|/Script/Engine.AudioComponent|SetSound (Variables|Default|GetCybird-4jianzhu-lead) (Variables|Default|GetSound)))