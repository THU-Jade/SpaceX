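; Player pawn that acts as an eight-note musical instrument on keys E through P, with a scripted video intro.
; Each key plays its note, nudges its mesh and lights a dynamic material created in the construction script.
; ForkCom blends the camera, possesses the pawn, shows a timed video, then animates the MP_Line collection for a Fourier effect.
; An NRT loudness visualizer for that line and four orbs is present but never bound.
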(event Custom|Playback0
  (params (PlayingSoundWave :type Sound%20Wave%20Object%20Reference) (PlaybackPercent :type Float%20%28single-precision%29))
  (bind _sound_nrt (Variables|Default|GetSound_NRT))
  (bind _duration (Variables|Default|GetDuration))
  (bind _returnvalue (* PlaybackPercent _duration))
  (bind _outloudness (Class|LoudnessNRT|GetNormalizedChannelLoudnessatTime _sound_nrt _returnvalue))
  (bind _returnvalue_2 (Math|Float|Power _outloudness 2.0))
  ;[1 1 1] 可视化部分
  (Rendering|Material|SetScalarParameterValue "/Game/Jade/Mat/MP_Line.MP_Line" "Loacation" _returnvalue_2 :!class /Script/Engine.KismetMaterialLibrary)
  (Transformation|SetRelativeScale3D (Variables|Default|GetP_ElectricOrb2) (Math|Conversions|ToVector(Float) _returnvalue_2)))

(event EventForkCom
  (bind _returnvalue (Game|GetPlayerController 0))
  (bind _self self)
  (bind _media (Variables|Default|GetMedia))
  ;[1 1 1] 切换摄像机控制权
  (Rendering|SetActorHiddenInGame false)
  (Game|Player|SetViewTargetwithBlend _returnvalue _self 3.0 "VTBlend_EaseInOut" 3.0 false)
  (Utilities|FlowControl|Delay 3.0)
  (Pawn|Possess _returnvalue _self)
  ;[1 1 1] 播放视频
  (Rendering|SetVisibility (Variables|Default|GetPlane) true false)
  (Media|MediaPlayer|OpenSource _media "/Game/Jade/MP4/TDMovieOut.TDMovieOut")
  (Media|MediaPlayer|Play _media :!class /Script/MediaAssets.MediaPlayer)
  (Utilities|FlowControl|Delay 41.0)
  (Rendering|SetVisibility (Variables|Default|GetPlane) false false)
  ;[1 1 1] 傅里叶变换动画
  (bind _新建轨道_0 (Timeline|时间轴 Play)
    (:Update
      (Rendering|Material|SetScalarParameterValue "/Game/Jade/Mat/MP_Line.MP_Line" "Loacation" (Math|Float|Lerp 0.0 1.0 _新建轨道_0) :!class /Script/Engine.KismetMaterialLibrary))))

(event EventBeginPlay
  ;[1 1 1] 可视化部分
)

(event Input|KeyboardEvents|T
  (params (Key :type Key%20Structure :default "None"))
  (bind _sm_fly2 (Variables|Default|GetSM_FLY2))
  (bind _m_mi (Variables|Default|GetM_mi))
  ;[1 1 1] mi
  (:Pressed
    (Rendering|Material|SetScalarParameterValue _m_mi "EM" 2.0 :!class /Script/Engine.MaterialInstanceDynamic)
    (Audio|PlaySound2D "/Game/Jade/Sound/8Sound/Falcon_01-03.Falcon_01-03" 1.0 1.0 0.0 0 0)
    (Transformation|SetRelativeLocation _sm_fly2 "0.000000,0.000000,1.000000" false false))
  (:Released
    (Rendering|Material|SetScalarParameterValue _m_mi "EM" 0.0 :!class /Script/Engine.MaterialInstanceDynamic)
    (Transformation|SetRelativeLocation _sm_fly2 "0, 0, 0" false false)))

(event Input|KeyboardEvents|Y
  (params (Key :type Key%20Structure :default "None"))
  (bind _m_fa (Variables|Default|GetM_fa))
  (bind _sm_fly3 (Variables|Default|GetSM_FLY3))
  ;[1 1 1] fa
  (:Pressed
    (Rendering|Material|SetScalarParameterValue _m_fa "EM" 2.0 :!class /Script/Engine.MaterialInstanceDynamic)
    (Audio|PlaySound2D "/Game/Jade/Sound/8Sound/Falcon_01-04.Falcon_01-04" 1.0 1.0 0.0 0 0)
    (Transformation|SetRelativeLocation _sm_fly3 "0.000000,0.000000,1.000000" false false))
  (:Released
    (Rendering|Material|SetScalarParameterValue _m_fa "EM" 0.0 :!class /Script/Engine.MaterialInstanceDynamic)
    (Transformation|SetRelativeLocation _sm_fly3 "0, 0, 0" false false)))

(event Input|KeyboardEvents|U
  (params (Key :type Key%20Structure :default "None"))
  (bind _m_so (Variables|Default|GetM_so))
  (bind _sm_fly4 (Variables|Default|GetSM_FLY4))
  ;[1 1 1] so
  (:Pressed
    (Rendering|Material|SetScalarParameterValue _m_so "EM" 2.0 :!class /Script/Engine.MaterialInstanceDynamic)
    (Audio|PlaySound2D "/Game/Jade/Sound/8Sound/Falcon_01-05.Falcon_01-05" 1.0 1.0 0.0 0 0)
    (Transformation|SetRelativeLocation _sm_fly4 "0.000000,0.000000,1.000000" false false))
  (:Released
    (Rendering|Material|SetScalarParameterValue _m_so "EM" 0.0 :!class /Script/Engine.MaterialInstanceDynamic)
    (Transformation|SetRelativeLocation _sm_fly4 "0, 0, 0" false false)))

(event Input|KeyboardEvents|I
  (params (Key :type Key%20Structure :default "None"))
  (bind _m_la (Variables|Default|GetM_la))
  (bind _sm_fly5 (Variables|Default|GetSM_FLY5))
  ;[1 1 1] la
  (:Pressed
    (Rendering|Material|SetScalarParameterValue _m_la "EM" 2.0 :!class /Script/Engine.MaterialInstanceDynamic)
    (Audio|PlaySound2D "/Game/Jade/Sound/8Sound/Falcon_01-06.Falcon_01-06" 1.0 1.0 0.0 0 0)
    (Transformation|SetRelativeLocation _sm_fly5 "0.000000,0.000000,1.000000" false false))
  (:Released
    (Rendering|Material|SetScalarParameterValue _m_la "EM" 0.0 :!class /Script/Engine.MaterialInstanceDynamic)
    (Transformation|SetRelativeLocation _sm_fly5 "0, 0, 0" false false)))

(event Input|KeyboardEvents|O
  (params (Key :type Key%20Structure :default "None"))
  (bind _m_xi (Variables|Default|GetM_xi))
  (bind _sm_fly6 (Variables|Default|GetSM_FLY6))
  ;[1 1 1] xi
  (:Pressed
    (Rendering|Material|SetScalarParameterValue _m_xi "EM" 2.0 :!class /Script/Engine.MaterialInstanceDynamic)
    (Audio|PlaySound2D "/Game/Jade/Sound/8Sound/Falcon_01-07.Falcon_01-07" 1.0 1.0 0.0 0 0)
    (Transformation|SetRelativeLocation _sm_fly6 "0.000000,0.000000,1.000000" false false))
  (:Released
    (Rendering|Material|SetScalarParameterValue _m_xi "EM" 0.0 :!class /Script/Engine.MaterialInstanceDynamic)
    (Transformation|SetRelativeLocation _sm_fly6 "0, 0, 0" false false)))

(event Input|KeyboardEvents|P
  (params (Key :type Key%20Structure :default "None"))
  (bind _m_do1 (Variables|Default|GetM_do1))
  (bind _sm_fly7 (Variables|Default|GetSM_FLY7))
  ;[1 1 1] do1
  (:Pressed
    (Rendering|Material|SetScalarParameterValue _m_do1 "EM" 2.0 :!class /Script/Engine.MaterialInstanceDynamic)
    (Audio|PlaySound2D "/Game/Jade/Sound/8Sound/Falcon_01-08.Falcon_01-08" 1.0 1.0 0.0 0 0)
    (Transformation|SetRelativeLocation _sm_fly7 "0.000000,0.000000,1.000000" false false))
  (:Released
    (Rendering|Material|SetScalarParameterValue _m_do1 "EM" 0.0 :!class /Script/Engine.MaterialInstanceDynamic)
    (Transformation|SetRelativeLocation _sm_fly7 "0, 0, 0" false false)))

(event Input|KeyboardEvents|E
  (params (Key :type Key%20Structure :default "None"))
  (bind _sm_fly (Variables|Default|GetSM_FLY))
  (bind _m_do (Variables|Default|GetM_do))
  ;[1 1 1] do0
  (:Pressed
    (Rendering|Material|SetScalarParameterValue _m_do "EM" 2.0 :!class /Script/Engine.MaterialInstanceDynamic)
    (Audio|PlaySound2D "/Game/Jade/Sound/8Sound/Falcon_01-01.Falcon_01-01" 1.0 1.0 0.0 0 0)
    (Transformation|SetRelativeLocation _sm_fly "0.000000,0.000000,1.000000" false false))
  (:Released
    (Rendering|Material|SetScalarParameterValue _m_do "EM" 0.0 :!class /Script/Engine.MaterialInstanceDynamic)
    (Transformation|SetRelativeLocation _sm_fly "0, 0, 0" false false)))

(event Input|KeyboardEvents|R
  (params (Key :type Key%20Structure :default "None"))
  (bind _sm_fly1 (Variables|Default|GetSM_FLY1))
  (bind _m_ri (Variables|Default|GetM_ri))
  ;[1 1 1] ri
  (:Pressed
    (Rendering|Material|SetScalarParameterValue _m_ri "EM" 2.0 :!class /Script/Engine.MaterialInstanceDynamic)
    (Audio|PlaySound2D "/Game/Jade/Sound/8Sound/Falcon_01-02.Falcon_01-02" 1.0 1.0 0.0 0 0)
    (Transformation|SetRelativeLocation _sm_fly1 "0.000000,0.000000,1.000000" false false))
  (:Released
    (Rendering|Material|SetScalarParameterValue _m_ri "EM" 0.0 :!class /Script/Engine.MaterialInstanceDynamic)
    (Transformation|SetRelativeLocation _sm_fly1 "0, 0, 0" false false)))

(fn ConstructionScript
  (bind _sound_nrt (Variables|Default|GetSound_NRT))
  (bind _sound (Variables|/Script/AudioAnalyzer.AudioAnalyzerNRT|GetSound _sound_nrt))
  (Utilities|FlowControl|Sequence
    (:then_0
      (bind _returnvalue (Rendering|Material|CreateDynamicMaterialInstance (Variables|Default|GetSM_FLY) 0 "/Game/Jade/Mat/Bright.Bright" "None" :!class /Script/Engine.PrimitiveComponent))
      (Variables|Default|SetM_do _returnvalue))
    (:then_1
      (bind _returnvalue_2 (Rendering|Material|CreateDynamicMaterialInstance (Variables|Default|GetSM_FLY1) 0 "/Game/Jade/Mat/Bright.Bright" "None" :!class /Script/Engine.PrimitiveComponent))
      (Variables|Default|SetM_ri _returnvalue_2))
    (:then_2
      (bind _returnvalue_3 (Rendering|Material|CreateDynamicMaterialInstance (Variables|Default|GetSM_FLY3) 0 "/Game/Jade/Mat/Bright.Bright" "None" :!class /Script/Engine.PrimitiveComponent))
      (Variables|Default|SetM_fa _returnvalue_3))
    (:then_3
      (bind _returnvalue_4 (Rendering|Material|CreateDynamicMaterialInstance (Variables|Default|GetSM_FLY2) 0 "/Game/Jade/Mat/Bright.Bright" "None" :!class /Script/Engine.PrimitiveComponent))
      (Variables|Default|SetM_mi _returnvalue_4))
    (:then_4
      (bind _returnvalue_5 (Rendering|Material|CreateDynamicMaterialInstance (Variables|Default|GetSM_FLY4) 0 "/Game/Jade/Mat/Bright.Bright" "None" :!class /Script/Engine.PrimitiveComponent))
      (Variables|Default|SetM_so _returnvalue_5))
    (:then_5
      (bind _returnvalue_6 (Rendering|Material|CreateDynamicMaterialInstance (Variables|Default|GetSM_FLY5) 0 "/Game/Jade/Mat/Bright.Bright" "None" :!class /Script/Engine.PrimitiveComponent))
      (Variables|Default|SetM_la _returnvalue_6))
    (:then_6
      (bind _returnvalue_7 (Rendering|Material|CreateDynamicMaterialInstance (Variables|Default|GetSM_FLY6) 0 "/Game/Jade/Mat/Bright.Bright" "None" :!class /Script/Engine.PrimitiveComponent))
      (Variables|Default|SetM_xi _returnvalue_7))
    (:then_7
      (bind _returnvalue_8 (Rendering|Material|CreateDynamicMaterialInstance (Variables|Default|GetSM_FLY7) 0 "/Game/Jade/Mat/Bright.Bright" "None" :!class /Script/Engine.PrimitiveComponent))
      (Variables|Default|SetM_do1 _returnvalue_8))
    (:then_8
      (Audio|Components|Audio|SetSound (Variables|Default|GetAudio) _sound)
      (Variables|Default|SetDuration (Variables|/Script/Engine.SoundBase|GetDuration _sound)))))