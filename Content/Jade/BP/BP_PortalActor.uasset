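; BP_PortalActor is a portal that moves the FirstPerson character to another portal when the character overlaps its Plane.
; It finds the destination as the first BP_PortalActor carrying the DoorNum tag.
; The character is placed at that portal's Arrow location, offset by ForwardM along the entered portal's forward vector, without sweep and without changing rotation.
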(event OnComponentBeginOverlap(Plane)
  (params (OverlappedComponent :type Primitive%20Component%20Object%20Reference) (OtherActor :type Actor%20Object%20Reference) (OtherComp :type Primitive%20Component%20Object%20Reference) (OtherBodyIndex :type Integer) (bFromSweep :type Boolean) (SweepResult :type Hit%20Result%20Structure%20%28by%20ref%29))
  (bind _asfirst_person (Utilities|Casting|CastToFirstPerson OtherActor))
  (bind _outactors (Actor|GetAllActorsOfClasswithTag "BP_PortalActor_C" (Variables|Default|GetDoor_Num)))
  (Transformation|SetActorLocation _asfirst_person (+ (Transformation|GetWorldLocation (Variables|BP_PortalActor_C|GetArrow (Utilities|Array|Get(acopy) _outactors))) (* (Math|Vector|GetForwardVector (Transformation|GetActorRotation)) (Variables|Default|GetForward_M))) false false))

(event EventBeginPlay)

(event Collision|EventActorBeginOverlap
  (params (OtherActor :type Actor%20Object%20Reference)))

(event EventTick
  (params (DeltaSeconds :type Float%20%28single-precision%29)))

(fn ConstructionScript)