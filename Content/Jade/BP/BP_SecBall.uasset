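; BP_SecBall is a trigger ball that hands the player over from the current level to Level_FixMoonMusic.
; When BP_ThirdPersonBall overlaps its sphere and AllowCol is set, it blends to NewCamera, hides the BP_PathTracer guides and plays the First_Second sequence.
; A delayed gate then lets Tick raise Ball_Bright in the MP_Line parameter collection every frame, while a longer delay times the level load.
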(event OnComponentBeginOverlap(Sphere)
  (params (OverlappedComponent :type Primitive%20Component%20Object%20Reference) (OtherActor :type Actor%20Object%20Reference) (OtherComp :type Primitive%20Component%20Object%20Reference) (OtherBodyIndex :type Integer) (bFromSweep :type Boolean) (SweepResult :type Hit%20Result%20Structure%20%28by%20ref%29))
  (if (Variables|Default|GetAllow_Col)
    (Utilities|Casting|CastToBP_ThirdPersonBall OtherActor)
    (Game|Player|SetViewTargetwithBlend (Game|GetPlayerController 0) (Variables|Default|GetNewCamera) 3.0 "VTBlend_EaseInOut" 2.0 true)
    ;[1 1 1] 隐藏引导
    (bind _outactors (Actor|GetAllActorsOfClass "/Game/PathTracer/Blueprints/BP_PathTracer.BP_PathTracer_C"))
    (Rendering|SetActorHiddenInGame _outactors true)
    (bind _returnvalue (Sequencer|Player|CreateLevelSequencePlayer "/Game/Sequence/First_Second.First_Second"))
    (Sequencer|Player|Play _returnvalue :!class /Script/MovieScene.MovieSceneSequencePlayer)
    (Utilities|FlowControl|Sequence
      (:then_0
        (Utilities|FlowControl|Delay 0.2)
        (Utilities|FlowControl|Gate true) ; enters at Open
      )
      (:then_1
        (Utilities|FlowControl|Delay 13.0)
        (Game|OpenLevel(byObjectReference) "/Game/level_FixMoonMusic.level_FixMoonMusic")))))

(event EventBeginPlay
  (Rendering|SetActorHiddenInGame false))

(event Collision|EventActorBeginOverlap
  (params (OtherActor :type Actor%20Object%20Reference)))

(event EventTick
  (params (DeltaSeconds :type Float%20%28single-precision%29))
  (Utilities|FlowControl|Gate true
    (:Exit
      (bind _output_get (Variables|Default|SetBall_Bright (+ (stale _output_get) 1.0)))
      (Rendering|Material|SetScalarParameterValue "/Game/Jade/Mat/MP_Line.MP_Line" "Ball_Bright" _output_get :!class /Script/Engine.KismetMaterialLibrary))))

(fn ConstructionScript)