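; BP_YinliBo is a gravitational-wave (yinli bo) trigger that BP_ThirdPersonBall catches by overlapping its Sphere.
; The construction script gives Sphere1 a dynamic light material, and the overlap plays a timeline that ramps its EM parameter.
; When the timeline finishes, it reveals the first ball actor's next hidden NBall component of four, then calls CatchYinliBoMessage on all ball actors.
; If all four are already visible, nothing further happens.
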(event OnComponentBeginOverlap(Sphere)
  (params (OverlappedComponent :type Primitive%20Component%20Object%20Reference) (OtherActor :type Actor%20Object%20Reference) (OtherComp :type Primitive%20Component%20Object%20Reference) (OtherBodyIndex :type Integer) (bFromSweep :type Boolean) (SweepResult :type Hit%20Result%20Structure%20%28by%20ref%29))
  (Utilities|Casting|CastToBP_ThirdPersonBall OtherActor)
  (bind _新建轨道_0 (Timeline|时间轴 Play)
    (:Update
      (Rendering|Material|SetScalarParameterValue (Variables|Default|GetA_Mat) "EM" (Math|Float|Lerp 0.0 1e+01 _新建轨道_0) :!class /Script/Engine.MaterialInstanceDynamic))
    (:Finished
      (bind _outactors (Actor|GetAllActorsOfClass "/Game/ThirdPerson/Blueprints/BP_ThirdPersonBall.BP_ThirdPersonBall_C"))
      (if (Rendering|IsVisible (Variables|/Game/ThirdPerson/Blueprints/BP_ThirdPersonBall.BP_ThirdPersonBall_C|GetN_Ball (Utilities|Array|Get(acopy) _outactors)))
        (if (Rendering|IsVisible (Variables|/Game/ThirdPerson/Blueprints/BP_ThirdPersonBall.BP_ThirdPersonBall_C|GetN_Ball1 (Utilities|Array|Get(acopy) _outactors)))
          (if (Rendering|IsVisible (Variables|/Game/ThirdPerson/Blueprints/BP_ThirdPersonBall.BP_ThirdPersonBall_C|GetN_Ball2 (Utilities|Array|Get(acopy) _outactors)))
            (if (not (Rendering|IsVisible (Variables|/Game/ThirdPerson/Blueprints/BP_ThirdPersonBall.BP_ThirdPersonBall_C|GetN_Ball3 (Utilities|Array|Get(acopy) _outactors))))
              (Rendering|SetVisibility (Variables|/Game/ThirdPerson/Blueprints/BP_ThirdPersonBall.BP_ThirdPersonBall_C|GetN_Ball3 (Utilities|Array|Get(acopy) _outactors)) true false)
              (Class|BWBall|CatchYinliBo(Message) _outactors :!label _label))
            (else
              (Rendering|SetVisibility (Variables|/Game/ThirdPerson/Blueprints/BP_ThirdPersonBall.BP_ThirdPersonBall_C|GetN_Ball2 (Utilities|Array|Get(acopy) _outactors)) true false)
              (goto _label)))
          (else
            (Rendering|SetVisibility (Variables|/Game/ThirdPerson/Blueprints/BP_ThirdPersonBall.BP_ThirdPersonBall_C|GetN_Ball1 (Utilities|Array|Get(acopy) _outactors)) true false)
            (goto _label)))
        (else
          (Rendering|SetVisibility (Variables|/Game/ThirdPerson/Blueprints/BP_ThirdPersonBall.BP_ThirdPersonBall_C|GetN_Ball (Utilities|Array|Get(acopy) _outactors)) true false)
          (goto _label))))))

(event EventBeginPlay)

(event Collision|EventActorBeginOverlap
  (params (OtherActor :type Actor%20Object%20Reference)))

(event EventTick
  (params (DeltaSeconds :type Float%20%28single-precision%29)))

(fn ConstructionScript
  (bind _returnvalue (Rendering|Material|CreateDynamicMaterialInstance (Variables|Default|GetSphere1) 0 "/Game/Jade/EasySpaceVFX/EasySpaceVFX/Aurora/Materials/M_Light_Inst.M_Light_Inst" "None" :!class /Script/Engine.PrimitiveComponent))
  (Variables|Default|SetA_Mat _returnvalue))