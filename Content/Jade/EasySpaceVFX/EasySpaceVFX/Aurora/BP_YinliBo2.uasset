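; BP_YinliBo2 is an aurora VFX trigger actor that reacts when the third-person character enters its sphere.
; The construction script creates a dynamic instance of M_Aurora_Inst on AuroraPlane.
; On overlap, a timeline drives the material's OP parameter between 1 and 0, apparently fading the aurora out.
; When the timeline finishes, it makes NBall2 visible on the first BP_ThirdPersonCharacter found in the level.
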(event OnComponentBeginOverlap(Sphere)
  (params (OverlappedComponent :type Primitive%20Component%20Object%20Reference) (OtherActor :type Actor%20Object%20Reference) (OtherComp :type Primitive%20Component%20Object%20Reference) (OtherBodyIndex :type Integer) (bFromSweep :type Boolean) (SweepResult :type Hit%20Result%20Structure%20%28by%20ref%29))
  (Utilities|Casting|CastToBP_ThirdPersonCharacter OtherActor)
  (bind _新建轨道_0 (Timeline|时间轴 Play)
    (:Update
      (Rendering|Material|SetScalarParameterValue (Variables|Default|GetA_Mat) "OP" (Math|Float|Lerp 1.0 0.0 _新建轨道_0) :!class /Script/Engine.MaterialInstanceDynamic))
    (:Finished
      (bind _outactors (Actor|GetAllActorsOfClass "/Game/ThirdPerson/Blueprints/BP_ThirdPersonCharacter.BP_ThirdPersonCharacter_C"))
      (Rendering|SetVisibility (Variables|/Game/ThirdPerson/Blueprints/BP_ThirdPersonCharacter.BP_ThirdPersonCharacter_C|GetN_Ball2 (Utilities|Array|Get(acopy) _outactors)) true false))))

(event EventBeginPlay)

(event Collision|EventActorBeginOverlap
  (params (OtherActor :type Actor%20Object%20Reference)))

(event EventTick
  (params (DeltaSeconds :type Float%20%28single-precision%29)))

(fn ConstructionScript
  (bind _returnvalue (Rendering|Material|CreateDynamicMaterialInstance (Variables|Default|GetAuroraPlane) 0 "/Game/Jade/EasySpaceVFX/EasySpaceVFX/Aurora/Materials/M_Aurora_Inst.M_Aurora_Inst" "None" :!class /Script/Engine.PrimitiveComponent))
  (Variables|Default|SetA_Mat _returnvalue))