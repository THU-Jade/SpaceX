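; BP_Fork is a fork pickup that bobs up and down via two timelines that restart each other in an endless loop.
; Its sphere overlap shows a press-E prompt to FirstPerson and opens a gate that lets the EFork event through, closing it on exit.
; EFork reveals the player's fork mesh, sets CanActive on every BP_ForkTower, hides the pickup, shows a Can_Active widget and destroys itself after a delay.
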(event OnComponentBeginOverlap(Sphere)
  (params (OverlappedComponent :type Primitive%20Component%20Object%20Reference) (OtherActor :type Actor%20Object%20Reference) (OtherComp :type Primitive%20Component%20Object%20Reference) (OtherBodyIndex :type Integer) (bFromSweep :type Boolean) (SweepResult :type Hit%20Result%20Structure%20%28by%20ref%29))
  (bind _asfirst_person (Utilities|Casting|CastToFirstPerson OtherActor))
  (bind _returnvalue (UserInterface|CreateWidget "/Game/Jade/Widget/PressE_Pick.PressE_Pick_C"))
  (UserInterface|Viewport|AddtoViewport _returnvalue 0)
  (Utilities|FlowControl|Gate true) ; enters at Open
)

(event OnComponentEndOverlap(Sphere)
  (params (OverlappedComponent :type Primitive%20Component%20Object%20Reference) (OtherActor :type Actor%20Object%20Reference) (OtherComp :type Primitive%20Component%20Object%20Reference) (OtherBodyIndex :type Integer))
  (Utilities|Casting|CastToFirstPerson OtherActor)
  (Viewport|RemoveAllWidgets)
  (Utilities|FlowControl|Gate true) ; enters at Close
)

(event EventBeginPlay
  (bind _sm_fork (Variables|Default|GetSM_Fork))
  (bind _新建轨道_0 (Timeline|时间轴 Play)
    (:Update
      (Transformation|SetRelativeLocation _sm_fork (Math|Vector|MakeVector 0.0 0.0 (Math|Float|Lerp -1e+01 1e+01 _新建轨道_0)) false false))
    (:Finished
      (bind _新建轨道_0_2 (Timeline|时间轴_0 PlayFromStart)
        (:Update
          (Transformation|SetRelativeLocation _sm_fork (Math|Vector|MakeVector 0.0 0.0 (Math|Float|Lerp 1e+01 -1e+01 _新建轨道_0_2)) false false))
        (:Finished
          (Timeline|时间轴 PlayFromStart))))))

(event EventEFork
  (Utilities|FlowControl|Gate true
    (:Exit
      (Rendering|SetVisibility (Variables|/Game/PUPI/Demo/Character/FirstPerson.FirstPerson_C|GetSM_Fork (stale OnComponentBeginOverlap(Sphere) _asfirst_person)) true false)
      (Viewport|RemoveAllWidgets)
      (bind _outactors (Actor|GetAllActorsOfClass "/Game/Jade/BP/BP_ForkTower.BP_ForkTower_C"))
      (for _array_element _outactors
        (Variables|/Game/Jade/BP/BP_ForkTower.BP_ForkTower_C|SetCan_Active _array_element true))
      (Rendering|SetActorHiddenInGame true)
      (bind _returnvalue (UserInterface|CreateWidget "/Game/Jade/Widget/Can_Active.Can_Active_C" (Game|GetPlayerController 0)))
      (UserInterface|Viewport|AddtoViewport _returnvalue 0)
      (Utilities|FlowControl|Delay 5.0)
      (Actor|DestroyActor))))

(fn ConstructionScript)