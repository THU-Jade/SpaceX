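; Pawn that works as a playable one-octave keyboard, mapping keys E through P along the top row to eight notes from do to high do.
; The construction script gives each of eight SMFLY meshes its own dynamic instance of the Bright material, one per note.
; Pressing a key raises that instance's EM parameter and plays the matching Falcon sound in 2D; releasing it resets EM to zero, leaving the sound untouched.
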(event EventBeginPlay)

(event Input|KeyboardEvents|T
  (params (Key :type Key%20Structure :default "None"))
  (bind _m_mi (Variables|Default|GetM_mi))
  ;[1 1 1] mi
  (:Pressed
    (Rendering|Material|SetScalarParameterValue _m_mi "EM" 2.0 :!class /Script/Engine.MaterialInstanceDynamic)
    (Audio|PlaySound2D "/Game/Jade/Sound/8Sound/Falcon_01-03.Falcon_01-03" 1.0 1.0 0.0 0 0))
  (:Released
    (Rendering|Material|SetScalarParameterValue _m_mi "EM" 0.0 :!class /Script/Engine.MaterialInstanceDynamic)))

(event Input|KeyboardEvents|Y
  (params (Key :type Key%20Structure :default "None"))
  (bind _m_fa (Variables|Default|GetM_fa))
  ;[1 1 1] fa
  (:Pressed
    (Rendering|Material|SetScalarParameterValue _m_fa "EM" 2.0 :!class /Script/Engine.MaterialInstanceDynamic)
    (Audio|PlaySound2D "/Game/Jade/Sound/8Sound/Falcon_01-04.Falcon_01-04" 1.0 1.0 0.0 0 0))
  (:Released
    (Rendering|Material|SetScalarParameterValue _m_fa "EM" 0.0 :!class /Script/Engine.MaterialInstanceDynamic)))

(event Input|KeyboardEvents|U
  (params (Key :type Key%20Structure :default "None"))
  (bind _m_so (Variables|Default|GetM_so))
  ;[1 1 1] so
  (:Pressed
    (Rendering|Material|SetScalarParameterValue _m_so "EM" 2.0 :!class /Script/Engine.MaterialInstanceDynamic)
    (Audio|PlaySound2D "/Game/Jade/Sound/8Sound/Falcon_01-05.Falcon_01-05" 1.0 1.0 0.0 0 0))
  (:Released
    (Rendering|Material|SetScalarParameterValue _m_so "EM" 0.0 :!class /Script/Engine.MaterialInstanceDynamic)))

(event Input|KeyboardEvents|I
  (params (Key :type Key%20Structure :default "None"))
  (bind _m_la (Variables|Default|GetM_la))
  ;[1 1 1] la
  (:Pressed
    (Rendering|Material|SetScalarParameterValue _m_la "EM" 2.0 :!class /Script/Engine.MaterialInstanceDynamic)
    (Audio|PlaySound2D "/Game/Jade/Sound/8Sound/Falcon_01-06.Falcon_01-06" 1.0 1.0 0.0 0 0))
  (:Released
    (Rendering|Material|SetScalarParameterValue _m_la "EM" 0.0 :!class /Script/Engine.MaterialInstanceDynamic)))

(event Input|KeyboardEvents|O
  (params (Key :type Key%20Structure :default "None"))
  (bind _m_xi (Variables|Default|GetM_xi))
  ;[1 1 1] xi
  (:Pressed
    (Rendering|Material|SetScalarParameterValue _m_xi "EM" 2.0 :!class /Script/Engine.MaterialInstanceDynamic)
    (Audio|PlaySound2D "/Game/Jade/Sound/8Sound/Falcon_01-07.Falcon_01-07" 1.0 1.0 0.0 0 0))
  (:Released
    (Rendering|Material|SetScalarParameterValue _m_xi "EM" 0.0 :!class /Script/Engine.MaterialInstanceDynamic)))

(event Input|KeyboardEvents|P
  (params (Key :type Key%20Structure :default "None"))
  (bind _m_do1 (Variables|Default|GetM_do1))
  ;[1 1 1] do1
  (:Pressed
    (Rendering|Material|SetScalarParameterValue _m_do1 "EM" 2.0 :!class /Script/Engine.MaterialInstanceDynamic)
    (Audio|PlaySound2D "/Game/Jade/Sound/8Sound/Falcon_01-08.Falcon_01-08" 1.0 1.0 0.0 0 0))
  (:Released
    (Rendering|Material|SetScalarParameterValue _m_do1 "EM" 0.0 :!class /Script/Engine.MaterialInstanceDynamic)))

(event Input|KeyboardEvents|E
  (params (Key :type Key%20Structure :default "None"))
  (bind _m_do (Variables|Default|GetM_do))
  ;[1 1 1] do0
  (:Pressed
    (Rendering|Material|SetScalarParameterValue _m_do "EM" 2.0 :!class /Script/Engine.MaterialInstanceDynamic)
    (Audio|PlaySound2D "/Game/Jade/Sound/8Sound/Falcon_01-01.Falcon_01-01" 1.0 1.0 0.0 0 0))
  (:Released
    (Rendering|Material|SetScalarParameterValue _m_do "EM" 0.0 :!class /Script/Engine.MaterialInstanceDynamic)))

(event Input|KeyboardEvents|R
  (params (Key :type Key%20Structure :default "None"))
  (bind _m_ri (Variables|Default|GetM_ri))
  ;[1 1 1] ri
  (:Pressed
    (Rendering|Material|SetScalarParameterValue _m_ri "EM" 2.0 :!class /Script/Engine.MaterialInstanceDynamic)
    (Audio|PlaySound2D "/Game/Jade/Sound/8Sound/Falcon_01-02.Falcon_01-02" 1.0 1.0 0.0 0 0))
  (:Released
    (Rendering|Material|SetScalarParameterValue _m_ri "EM" 0.0 :!class /Script/Engine.MaterialInstanceDynamic)))

(fn ConstructionScript
  (Utilities|FlowControl|Sequence
    (:then_0
      (bind _returnvalue (Rendering|Material|CreateDynamicMaterialInstance (Variables|Default|GetSM_FLY) 0 "/Game/Jade/Mesh/Bright.Bright" "None" :!class /Script/Engine.PrimitiveComponent))
      (Variables|Default|SetM_do _returnvalue))
    (:then_1
      (bind _returnvalue_2 (Rendering|Material|CreateDynamicMaterialInstance (Variables|Default|GetSM_FLY1) 0 "/Game/Jade/Mesh/Bright.Bright" "None" :!class /Script/Engine.PrimitiveComponent))
      (Variables|Default|SetM_ri _returnvalue_2))
    (:then_2
      (bind _returnvalue_3 (Rendering|Material|CreateDynamicMaterialInstance (Variables|Default|GetSM_FLY3) 0 "/Game/Jade/Mesh/Bright.Bright" "None" :!class /Script/Engine.PrimitiveComponent))
      (Variables|Default|SetM_fa _returnvalue_3))
    (:then_3
      (bind _returnvalue_4 (Rendering|Material|CreateDynamicMaterialInstance (Variables|Default|GetSM_FLY2) 0 "/Game/Jade/Mesh/Bright.Bright" "None" :!class /Script/Engine.PrimitiveComponent))
      (Variables|Default|SetM_mi _returnvalue_4))
    (:then_4
      (bind _returnvalue_5 (Rendering|Material|CreateDynamicMaterialInstance (Variables|Default|GetSM_FLY4) 0 "/Game/Jade/Mesh/Bright.Bright" "None" :!class /Script/Engine.PrimitiveComponent))
      (Variables|Default|SetM_so _returnvalue_5))
    (:then_5
      (bind _returnvalue_6 (Rendering|Material|CreateDynamicMaterialInstance (Variables|Default|GetSM_FLY5) 0 "/Game/Jade/Mesh/Bright.Bright" "None" :!class /Script/Engine.PrimitiveComponent))
      (Variables|Default|SetM_la _returnvalue_6))
    (:then_6
      (bind _returnvalue_7 (Rendering|Material|CreateDynamicMaterialInstance (Variables|Default|GetSM_FLY6) 0 "/Game/Jade/Mesh/Bright.Bright" "None" :!class /Script/Engine.PrimitiveComponent))
      (Variables|Default|SetM_xi _returnvalue_7))
    (:then_7
      (bind _returnvalue_8 (Rendering|Material|CreateDynamicMaterialInstance (Variables|Default|GetSM_FLY7) 0 "/Game/Jade/Mesh/Bright.Bright" "None" :!class /Script/Engine.PrimitiveComponent))
      (Variables|Default|SetM_do1 _returnvalue_8))))