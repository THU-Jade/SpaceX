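; Asteroid field actor that scatters four asteroid meshes in spherical, globular clusters using instanced static meshes.
; The construction script assigns the meshes, then each loop places one cluster per mesh at a random offset, with a quarter of the asteroid count.
; BPF_AsteroidCluster adds randomly rotated, scaled instances, using power-curved random radii like the cluster placement to control density.
; Randomness is unseeded, and the default-or-custom material branch is disconnected.
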(event EventBeginPlay)

(event Collision|EventActorBeginOverlap
  (params (OtherActor :type Actor%20Object%20Reference)))

(event EventTick
  (params (DeltaSeconds :type Float%20%28single-precision%29)))

(fn ConstructionScript
  (bind _returnvalue (Math|Random|RandomUnitVector))
  (bind _returnvalue_2 (Math|Random|RandomFloatinRange 0.0 1.0))
  (bind _clusters_distance (Variables|Clusters|GetClusters%20Distance))
  (bind _clusters_distance_distribution (Variables|Clusters|GetClusters%20Distance%20Distribution))
  (bind _returnvalue_3 (Math|Float|Power _returnvalue_2 _clusters_distance_distribution))
  (bind _returnvalue_4 (* _clusters_distance _returnvalue_3))
  (bind _returnvalue_5 (* _returnvalue _returnvalue_4))
  (Components|StaticMesh|SetStaticMesh (Variables|Default|GetISM_Asteroid_1) (Variables|StaticMeshes|GetSM%201))
  (Components|StaticMesh|SetStaticMesh (Variables|Default|GetISM_Asteroid_2) (Variables|StaticMeshes|GetSM%202))
  (Components|StaticMesh|SetStaticMesh (Variables|Default|GetISM_Asteroid_3) (Variables|StaticMeshes|GetSM%203))
  (Components|StaticMesh|SetStaticMesh (Variables|Default|GetISM_Asteroid_4) (Variables|StaticMeshes|GetSM%204))
  (for _index (range 0 (- (Variables|Clusters|GetNumber%20of%20Clusters) 1))
    (CallFunction|BPFAsteroidCluster (Variables|Default|GetISM_Asteroid_1) _returnvalue_5 (/ (Variables|Asteroids|GetNumber%20of%20Asteroids) 4) (Variables|Asteroids|GetAsteroid%20Distance) (Variables|Asteroids|GetAsteroid%20Distance%20Distribution) (Variables|Asteroids|GetAsteroid%20Scale) (Variables|Asteroids|GetAsteroid%20Scale%20Variation%20Fraction))
    (CallFunction|BPFAsteroidCluster (Variables|Default|GetISM_Asteroid_2) _returnvalue_5 (/ (Variables|Asteroids|GetNumber%20of%20Asteroids) 4) (Variables|Asteroids|GetAsteroid%20Distance) (Variables|Asteroids|GetAsteroid%20Distance%20Distribution) (Variables|Asteroids|GetAsteroid%20Scale) (Variables|Asteroids|GetAsteroid%20Scale%20Variation%20Fraction))
    (CallFunction|BPFAsteroidCluster (Variables|Default|GetISM_Asteroid_3) _returnvalue_5 (/ (Variables|Asteroids|GetNumber%20of%20Asteroids) 4) (Variables|Asteroids|GetAsteroid%20Distance) (Variables|Asteroids|GetAsteroid%20Distance%20Distribution) (Variables|Asteroids|GetAsteroid%20Scale) (Variables|Asteroids|GetAsteroid%20Scale%20Variation%20Fraction))
    (CallFunction|BPFAsteroidCluster (Variables|Default|GetISM_Asteroid_4) _returnvalue_5 (/ (Variables|Asteroids|GetNumber%20of%20Asteroids) 4) (Variables|Asteroids|GetAsteroid%20Distance) (Variables|Asteroids|GetAsteroid%20Distance%20Distribution) (Variables|Asteroids|GetAsteroid%20Scale) (Variables|Asteroids|GetAsteroid%20Scale%20Variation%20Fraction))))

(fn BPFAsteroidCluster
  (params (Instanced%20Static%20Mesh :type Instanced%20Static%20Mesh%20Component%20Object%20Reference) (Cluster%20Location :type Vector) (Number%20Of%20Asteroids :type Integer) (Asteroids%20Distance :type Float%20%28double-precision%29) (Asteroids%20Distance%20Distribution :type Float%20%28double-precision%29) (Asteroid%20Scale :type Float%20%28double-precision%29) (Asteroid%20Scale%20Variation :type Float%20%28double-precision%29))
  (for _index (range 0 (- Number%20Of%20Asteroids 1))
    (Components|InstancedStaticMesh|AddInstance Instanced%20Static%20Mesh (Math|Transform|MakeTransform (+ Cluster%20Location (* (Math|Random|RandomUnitVector) (* Asteroids%20Distance (Math|Float|Power (Math|Random|RandomFloatinRange 0.0 1.0) Asteroids%20Distance%20Distribution)))) (Math|Random|RandomRotator true) (Math|Conversions|ToVector(Float) (* Asteroid%20Scale (Math|Random|RandomFloatinRange (/ 1.0 Asteroid%20Scale%20Variation) 1.0)))) false))
  (return))